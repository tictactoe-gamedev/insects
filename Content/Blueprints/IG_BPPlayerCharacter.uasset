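; Player character Blueprint for a mouse-aimed, likely top-down, control scheme using Enhanced Input.
; BeginPlay adds the main mapping context and shows the mouse cursor.
; Tick traces the Visibility channel under the cursor and sets control rotation yaw to face the hit point.
; The PlayerMove action feeds normalized world-space X/Y movement input scaled by a move speed variable, independent of facing.
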(event Input|EnhancedActionEvents|EnhancedInputActionPlayerMove
  (params (ActionValue :type Vector%202D%20Structure) (ElapsedSeconds :type Float%20%28double-precision%29) (TriggeredSeconds :type Float%20%28double-precision%29) (InputAction :type Input%20Action%20Object%20Reference :default "/Game/Blueprints/Inputs/PlayerMove.PlayerMove"))
  ;[0.2172 1 0.2027 1 32] Player Movement
  (Pawn|Input|AddMovementInput (Math|Vector|Normalize (Math|Vector|MakeVector (.x ActionValue) (.y ActionValue) 0.0)) (Variables|Default|GetPlayerMoveSpeed) false))

(event EventBeginPlay
  (Utilities|FlowControl|Sequence
    (:then_0
      ;[0.9577 0.3385 1 1 32] Create Control Mapping
      (bind _asplayer_controller (Utilities|Casting|CastToPlayerController (Pawn|GetController)))
      (Input|AddMappingContext (PlayerController|LocalPlayerSubsystems|GetEnhancedInputLocalPlayerSubsystem _asplayer_controller) "/Game/Blueprints/Inputs/PlayerMainContext.PlayerMainContext" 0 "(bIgnoreAllPressedKeysUntilRelease=True,bForceImmediately=False,bNotifyUserSettings=False)"))
    (:then_1
      (Variables|/Script/Engine.PlayerController|SetbShowMouseCursor (Game|GetPlayerController 0) true))))

(event EventTick
  (params (DeltaSeconds :type Float%20%28single-precision%29))
  (bind _returnvalue (Game|GetPlayerController 0))
  (bind _hitresult (Game|Player|GetHitResultUnderCursorbyChannel _returnvalue "TraceTypeQuery1" false))
  (if (.bblockinghit _hitresult)
    (Pawn|SetControlRotation _returnvalue (Math|Rotator|MakeRotator 0.0 0.0 (.yaw (Math|Rotator|FindLookatRotation (Transformation|GetActorLocation) (.impactpoint _hitresult)))))))

(fn ConstructionScript)