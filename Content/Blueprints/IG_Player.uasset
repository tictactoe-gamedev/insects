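; IG_Player is the player character Blueprint for mouse-aimed melee combat.
; Each tick it traces under the cursor and yaws the controller to face that point, with the cursor shown from BeginPlay.
; The PlayerAttack input plays a montage whose notify window sets an Attacking flag and clears hit detection at the start.
; While Attacking, Tick runs DoHitDetection and applies PlayerDamage to the returned actor.
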(event Input|EnhancedActionEvents|EnhancedInputActionPlayerAttack
  (params (ActionValue :type Boolean) (ElapsedSeconds :type Float%20%28double-precision%29) (TriggeredSeconds :type Float%20%28double-precision%29) (InputAction :type Input%20Action%20Object%20Reference :default "/Game/Blueprints/Inputs/PlayerAttack.PlayerAttack"))
  (if false
    _
    (else
      _))
  (Animation|Montage|PlayMontage (Variables|Character|GetMesh) "/Game/Meshes/Boxman/IG_PlayerAnimMontage.IG_PlayerAnimMontage"
    (:then
      (Class|IGPlayerCharacter|ClearHitDetection))
    (:OnCompleted
      (Variables|Default|SetAttacking false :!label _label))
    (:OnInterrupted
      (goto _label))
    (:OnNotifyBegin
      (bind _output_get (Variables|Default|SetAttacking true)))
    (:OnNotifyEnd
      (goto _label))))

(event EventBeginPlay
  (Utilities|FlowControl|Sequence
    (:then_1
      (Variables|/Script/Engine.PlayerController|SetbShowMouseCursor (Game|GetPlayerController 0) true))))

(event EventTick
  (params (DeltaSeconds :type Float%20%28single-precision%29))
  (bind _returnvalue (Game|GetPlayerController 0))
  (bind _hitresult (Game|Player|GetHitResultUnderCursorbyChannel _returnvalue "TraceTypeQuery1" false))
  (Utilities|FlowControl|Sequence
    (:then_0
      ;[0 0.07053 1 1 32] Rotate to Cursor
      (if (.bblockinghit _hitresult)
        (Pawn|SetControlRotation _returnvalue (Math|Rotator|MakeRotator 0.0 0.0 (.yaw (Math|Rotator|FindLookatRotation (Transformation|GetActorLocation) (.impactpoint _hitresult)))))))
    (:then_1
      (if (stale Input|EnhancedActionEvents|EnhancedInputActionPlayerAttack _output_get)
        (bind _returnvalue_2 (Class|IGPlayerCharacter|DoHitDetection))
        (Game|Damage|ApplyDamage _returnvalue_2 (Variables|Default|GetPlayerDamage) (Pawn|GetController) self)))))

(fn ConstructionScript)